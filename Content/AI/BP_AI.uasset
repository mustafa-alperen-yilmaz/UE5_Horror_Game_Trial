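; AI character Blueprint that detects the player and performs a melee shove attack.
; Pawn sensing sets the seeingPlayer Blackboard key to true for Player-tagged pawns, and this graph never clears it.
; AttackPlayer plays a push montage behind an Attacking guard, then on completion sphere-traces for pawns and damages the hit actor.
; The trace's End omits the attack point's location, so it lands near world origin.
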(event `self.PawnSensing.OnSeePawn`
  (params (Pawn :type "Pawn Object Reference"))
  ;[0 0 0] Seeing Player
  (if (`self.ActorHasTag` Pawn "Player")
    (`BlackboardComponent.SetValueAsBool` (`AIBlueprintHelperLibrary.GetBlackboard` (`AIBlueprintHelperLibrary.GetAIController` self)) "seeingPlayer" true)))

(event `Attack Player`
  (bind _attack_trace_point (`self.Attack Trace Point`))
  (bind _returnvalue (* (`KismetMathLibrary.GetForwardVector` (`SceneComponent.K2_GetComponentRotation` _attack_trace_point)) 70.0))
  ;[0 0 0] Attack
  (if (not (`self.Attacking`))
    (set `self.Attacking` true)
    (`|PlayMontage` (`self.Mesh`) "/Game/AI/Paired_PushShove_Att_Montage.Paired_PushShove_Att_Montage"
      (:`OnCompleted`
        (set `self.Attacking` false)
        (bind (_outhit _returnvalue_2) (`KismetSystemLibrary.SphereTraceSingleForObjects` :`Start` (+ (`SceneComponent.K2_GetComponentLocation` _attack_trace_point) _returnvalue) :`End` _returnvalue :`Radius` 25.0 :`ObjectTypes` (`|MakeArray` "ObjectTypeQuery3" :!type "EObjectTypeQuery Enum") :`DrawDebugType` "ForDuration"))
        (if _returnvalue_2
          (`GameplayStatics.ApplyDamage` (`.HitActor` (`GameplayStatics.BreakHitResult` _outhit)) 10.0))))))

(fn `UserConstructionScript`)